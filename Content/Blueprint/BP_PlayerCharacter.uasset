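; BP_PlayerCharacter is the player character Blueprint, which equips a BP_THS1 actor, apparently a weapon, when play begins.
; After the parent BeginPlay, it spawns BP_THS1 and attaches it to the LeftWeapon component at hand_lSocket, snapping location, rotation and scale.
; Overlap and Tick events are disabled stubs, and the construction script only calls its parent.
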(event `self.ReceiveBeginPlay`
  (`parent.ReceiveBeginPlay`)
  (bind _returnvalue (`|SpawnActorFromClass` "/Game/Blueprint/Weapon/BP_THS1.BP_THS1_C" (`KismetMathLibrary.MakeTransform` (0.0 0.0 0.0)) "AlwaysSpawn" "OverrideRootScale" null null))
  (`self.K2_AttachToComponent` _returnvalue (`self.LeftWeapon`) "hand_lSocket" "SnapToTarget" "SnapToTarget" "SnapToTarget" true))

(fn `UserConstructionScript`
  (`parent.UserConstructionScript`))